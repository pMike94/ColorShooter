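; Game logic actor that runs enemy wave escalation and ends the game when no BP_Generator remains, showing HUD_End.
; SpawnEnemies and EnemyLoop form an endless random-delay loop, spawning BP_Enemy at a random point within a growing range of activated spawn points.
; Looping timers count game time, raise EnemySpeed, shrink the maximum spawn delay until it drops below a floor, and divide ExtraSpawnChance, which is not read here.
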(event Custom|ChangeSpawnChance
  ;[1 1 1] Increase Chance of Multiple Spawns over Time
  (Variables|Default|SetExtraSpawnChance (/ (Variables|Default|GetExtraSpawnChance) 1.2)))

(event Custom|CheckGeneratorNumber
  ;[1 1 1] Check if there is still a Generator LEft
  (bind _outactors (Actor|GetAllActorsOfClass "/Game/Blueprints/BP_Generator.BP_Generator_C"))
  (bind _output_get (Variables|Default|SetGeneratorNumber (Utilities|Array|Length _outactors)))
  (if (== _output_get 0)
    (Viewport|RemoveAllWidgets)
    (bind _returnvalue (UserInterface|CreateWidget "/Game/Widgets/HUD_End.HUD_End_C" (Game|GetPlayerController 0)))
    (UserInterface|Viewport|AddtoViewport _returnvalue 0)
    (Variables|Default|SetGameOver true)))

(event Custom|ChangeSpeed
  ;[1 1 1] Increase Speed of Enemies over Time
  (Variables|Default|SetEnemySpeed (* (Variables|Default|GetEnemySpeed) 1.05)))

(event Custom|ActivateEnemySpawn
  ;[1 1 1] Activate Enemy Spawn Points
  (Utilities|Time|SetTimerbyFunctionName 0 "ActivateEnemySpawnPoints" (Variables|Default|GetSpawnPointFrequency) true))

(event Custom|EnemyLoop
  ;[1 1 1] Loop Enemy Spawn Randomly
  (Utilities|FlowControl|Delay (Math|Random|RandomFloatinRange (Variables|Default|GetSpawnRateMin) (Variables|Default|GetSpawnRateMax)))
  (CallFunction|SpawnEnemies))

(event EventBeginPlay
  (Utilities|Time|SetTimerbyFunctionName 0 "SetTime" 1.0 true)
  ;[1 1 1] Get all possible Spawnpoints
  (bind _outactors (Actor|GetAllActorsOfClass "/Game/Blueprints/BP_EnemySpawnPoint.BP_EnemySpawnPoint_C"))
  (Variables|Default|SetSpawnPoints _outactors)
  ;[1 1 1] Increase Speed of Enemies over Time
  (Utilities|Time|SetTimerbyEvent (delegate Custom|ChangeSpeed) 1e+01 true)
  ;[1 1 1] Increase Chance of Multiple Spawns over Time
  (Utilities|Time|SetTimerbyEvent (delegate Custom|ChangeSpawnChance) 1e+01 true)
  (Utilities|FlowControl|Delay 5.0)
  (Utilities|Time|SetTimerbyFunctionName 0 "ReduceMaxSpawnRate" (Variables|Default|GetSpawnrateAmplifySeconds) true)
  (CallFunction|SpawnEnemies)
  (CallFunction|ActivateEnemySpawn)
  (Actor|GetAllActorsOfClass "/Script/Engine.Light"))

(fn ConstructionScript)

(fn SetTime
  (Math|Integer|IncrementInt (Variables|Default|GetTime)))

(fn SpawnEnemies
  (bind _activatedspawnpoints (Variables|Default|GetActivatedSpawnPoints))
  (bind _returnvalue (Math|Random|RandomIntegerinRange 0 _activatedspawnpoints))
  ;[1 1 1] Set A Random Spawn Point in the Level
  (Variables|Default|SetSpawnPointID _returnvalue)
  (Variables|Default|SetEnemySpawnPoint (Utilities|Array|Get(acopy) (Variables|Default|GetSpawnPoints) _returnvalue))
  (Game|SpawnActorfromClass "/Game/Blueprints/Enemies/BP_Enemy.BP_Enemy_C" (Transformation|GetActorTransform (Variables|Default|GetEnemySpawnPoint)) "Undefined" 0 0)
  (CallFunction|EnemyLoop))

(fn ActivateEnemySpawnPoints
  (Variables|Default|SetActivatedSpawnPoints (+ (Variables|Default|GetActivatedSpawnPoints) 1)))

(fn ReduceMaxSpawnRate
  (if (< (Variables|Default|GetSpawnRateMax) 2.3)
    (Utilities|Time|ClearTimerbyFunctionName 0 "ReduceMaxSpawnRate")
    (else
      (Variables|Default|SetSpawnRateMax (/ (Variables|Default|GetSpawnRateMax) 1.1)))))