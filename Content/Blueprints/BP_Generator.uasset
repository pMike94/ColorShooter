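; BP_Generator is a damageable objective actor that loses one health each time a BP_Enemy overlaps it, destroying that enemy.
; It shows its current health on a text render.
; On its last hit it destroys itself and tells enemy AI controllers targeting it to search for a new target.
; Each hit also asks BP_GameLogic, found at BeginPlay, to check the generator count.
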(event EventBeginPlay
  (Variables|Default|SetCurrentHealth (Variables|Default|GetMaxHealth))
  ;[1 1 1] Get Game Logic
  (bind _outactors (Actor|GetAllActorsOfClass "/Game/Blueprints/BP_GameLogic.BP_GameLogic_C"))
  (Variables|Default|SetGameLogic (Utilities|Array|Get(acopy) _outactors))
  (Rendering|Components|TextRender|SetText (Variables|Default|GetTextRender) (Utilities|Text|ToText(Integer) (Variables|Default|GetCurrentHealth))))

(event Collision|EventActorBeginOverlap
  (params (OtherActor :type Actor%20Object%20Reference))
  ;[1 1 1] Check if Overlapping Generator has only One Life Left
  (bind _asbp_enemy (Utilities|Casting|CastToBP_Enemy OtherActor))
  (if (== (Variables|Default|GetCurrentHealth) 1)
    (Actor|DestroyActor _asbp_enemy)
    ;[1 1 1] If yes Destroy it
    (Actor|DestroyActor)
    ;[1 1 1] AI search a new Target after Destruction
    (bind _outactors (Actor|GetAllActorsOfClass "/Game/Blueprints/Enemies/BP_Enemy.BP_Enemy_C"))
    (bind _array_element (Utilities|Array|ForEachLoopwithBreak _outactors)
      (:LoopBody
        (bind _asai_con (Utilities|Casting|CastToAI_CON (Pawn|GetController _array_element)))
        (if (== (Variables|/Game/Blueprints/Enemies/AI_CON.AI_CON_C|GetTarget _asai_con) self)
          (Default|SearchforTarget _asai_con)))
      (:Completed
        (Default|CheckGeneratorNumber (Variables|Default|GetGameLogic))))
    (else
      ;[1 1 1] If not take away one Life
      (Math|Integer|DecrementInt (Variables|Default|GetCurrentHealth)
        (:%20%20
          (Actor|DestroyActor _asbp_enemy)
          (Default|CheckGeneratorNumber (Variables|Default|GetGameLogic))
          (Rendering|Components|TextRender|SetText (Variables|Default|GetTextRender) (Utilities|Text|ToText(Integer) (Variables|Default|GetCurrentHealth))))))))

(fn ConstructionScript)