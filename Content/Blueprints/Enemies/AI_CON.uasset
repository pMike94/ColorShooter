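; Enemy AI controller that sends its controlled pawn toward the nearest generator in the level.
; Shortly after BeginPlay, a one-time search loops over all BP_Generator actors and stores the closest by straight-line distance as the target.
; Tick then reissues a simple move-to-actor toward that target every frame, without searching again.
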(event Custom|SearchForTarget
  ;[1 1 1] Get All Generators in Level
  (bind _outactors (Actor|GetAllActorsOfClass "/Game/Blueprints/BP_Generator.BP_Generator_C"))
  (Variables|Default|SetDistance 1e+09)
  ;[1 1 1] For Each Generator Check Distance between Gen/Enemy. If A Distance is lower, than the one thats Set. Set the new Distance
  (for _array_element _outactors
    (if (< (Math|Vector|VectorLength (- (Transformation|GetActorLocation _array_element) (Transformation|GetActorLocation (Pawn|GetControlledPawn)))) (Variables|Default|GetDistance))
      (Variables|Default|SetDistance (Math|Vector|VectorLength (- (Transformation|GetActorLocation _array_element) (Transformation|GetActorLocation (Pawn|GetControlledPawn)))))
      ;[1 1 1] Set Target to the one with the lowest Distance
      (Variables|Default|SetTarget _array_element))))

(event EventBeginPlay
  (Utilities|FlowControl|Delay 0.2)
  (CallFunction|SearchforTarget))

(event EventTick
  (params (DeltaSeconds :type Float%20%28single-precision%29))
  ;[1 1 1] Move Enemy to Generator
  (AI|Navigation|SimpleMovetoActor self (Variables|Default|GetTarget)))

(fn ConstructionScript)