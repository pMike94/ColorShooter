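; Drone enemy that takes a random red, yellow or blue color on spawn and can only be destroyed by a projectile of the same color.
; BeginPlay spawns its controller, reads speed from BP_GameLogic and tints a dynamic material and hover particle.
; A matching hit unpossesses it, shatters the destructible mesh and turns off emissive.
; An Alive flag stops debris hits from re-awarding the player coins and ammo before delayed cleanup.
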(event Collision|EventHit
  (params (MyComp :type Primitive%20Component%20Object%20Reference) (Other :type Actor%20Object%20Reference) (OtherComp :type Primitive%20Component%20Object%20Reference) (bSelfMoved :type Boolean) (HitLocation :type Vector :default "0, 0, 0") (HitNormal :type Vector :default "0, 0, 0") (NormalImpulse :type Vector :default "0, 0, 0") (Hit :type Hit%20Result%20Structure%20%28by%20ref%29))
  (bind _owncolor (Variables|Default|GetOwnColor))
  ;[1 1 1] Projectile Hits Enemy
  (bind _asbp_projectile (Utilities|Casting|CastToBP_Projectile Other))
  (if (Math|Boolean|ORBoolean (and (Variables|/Game/Blueprints/BP_Projectile.BP_Projectile_C|GetisRed _asbp_projectile) (== _owncolor 0)) (and (Variables|/Game/Blueprints/BP_Projectile.BP_Projectile_C|GetisYellow _asbp_projectile) (== _owncolor 1)) (and (Variables|/Game/Blueprints/BP_Projectile.BP_Projectile_C|GetisBlue _asbp_projectile) (== _owncolor 2)))
    (Components|DestroyComponent (Variables|Default|GetP_Hover))
    (Pawn|UnPossess (AI|GetAIController self))
    (Components|DestroyComponent (Variables|Collision|GetCapsuleComponent))
    (Class|DestructibleComponent|ApplyDamage (Variables|Default|GetDestructible) 1e+02 HitLocation HitNormal 1e+03)
    (Rendering|Material|SetScalarParameterValue (Variables|Default|GetDynaMat) "HasEmissive" 0.0 :!class /Script/Engine.MaterialInstanceDynamic)
    (Utilities|FlowControl|Delay 0.2)
    (Collision|SetCollisionResponsetoChannel (Variables|Default|GetDestructible) "ECC_Pawn" "ECR_Ignore")
    ;;[1 1 1] Prevent from getting Points by Shooting the Debris
    (if (Variables|Default|GetAlive)
      (Default|GetCoins (Variables|Default|GetPlayer))
      (Default|GetAmmo (Variables|Default|GetPlayer))
      (Variables|Default|SetAlive false)
      (Utilities|FlowControl|Delay 1e+01)
      (Actor|DestroyActor))))

(event EventBeginPlay
  (Pawn|SpawnDefaultController)
  ;[1 1 1] Get Speed from Game Logic
  (bind _outactors (Actor|GetAllActorsOfClass "/Game/Blueprints/BP_GameLogic.BP_GameLogic_C"))
  (Variables|/Script/Engine.CharacterMovementComponent|SetMaxWalkSpeed (Variables|Character|GetCharacterMovement) (Variables|/Game/Blueprints/BP_GameLogic.BP_GameLogic_C|GetEnemySpeed (Utilities|Array|Get(acopy) _outactors)))
  ;[1 1 1] Save Player as Variable
  (bind _outactors_2 (Actor|GetAllActorsOfClass "/Game/Blueprints/BP_Character.BP_Character_C"))
  (Variables|Default|SetPlayer (Utilities|Array|Get(acopy) _outactors_2))
  (bind _returnvalue (Rendering|Material|CreateDynamicMaterialInstance (Variables|Default|GetDestructible) 0 "/Game/Materials/Enemies/MI_Drone.MI_Drone" :!class /Script/Engine.PrimitiveComponent))
  (Variables|Default|SetDynaMat _returnvalue)
  (CallFunction|SetColor)
  (Variables|Default|SetAlive true))

(fn ConstructionScript)

(fn SetColor
  (bind _colred (Variables|Default|GetColRed))
  (bind _colyellow (Variables|Default|GetColYellow))
  (bind _colblue (Variables|Default|GetColBlue))
  ;[1 1 1] Set a Random ColorID for the Enemy on Spawn
  (Variables|Default|SetOwnColor (Math|Conversions|ToByte(Integer) (Math|Random|RandomIntegerinRange 0 2)))
  ;[1 1 1] Check if Color ID of Enemy is 0
  (if (== (Variables|Default|GetOwnColor) 0)
    ;[1 0 0.04693] If yes set Material and Particle to Red
    (Rendering|Material|SetVectorParameterValue (Variables|Default|GetDynaMat) "Color_G" _colred :!class /Script/Engine.MaterialInstanceDynamic)
    (Effects|Components|ParticleSystem|SetColorParameter (Variables|Default|GetP_Hover) "Color" _colred)
    (else
      ;[1 1 1] Check if ColorID of Enemy is 1
      (if (== (Variables|Default|GetOwnColor) 1)
        ;[1 0.8886 0] If Yes set Material to Yellow
        (Rendering|Material|SetVectorParameterValue (Variables|Default|GetDynaMat) "Color_G" _colyellow :!class /Script/Engine.MaterialInstanceDynamic)
        (Effects|Components|ParticleSystem|SetColorParameter (Variables|Default|GetP_Hover) "Color" _colyellow)
        (else
          ;[0 0.3096 1] If Not set Material to Blue
          (Rendering|Material|SetVectorParameterValue (Variables|Default|GetDynaMat) "Color_G" _colblue :!class /Script/Engine.MaterialInstanceDynamic)
          (Effects|Components|ParticleSystem|SetColorParameter (Variables|Default|GetP_Hover) "Color" _colblue))))))