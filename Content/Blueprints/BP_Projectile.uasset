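; BP_Projectile is a colored projectile that takes on the player's current color when it spawns.
; On BeginPlay it creates a dynamic material instance on its sphere, finds the first BP_Character and runs ChangeColor.
; ChangeColor reads the player's red, yellow or blue flag, sets the matching flag on itself and tints the material's Color parameter.
; On hit, it destroys itself after a very short delay.
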(event EventBeginPlay
  ;[1 1 1] Begin Play
  ;;[1 1 1] Create Dyna Mat Instance
  (bind _returnvalue (Rendering|Material|CreateDynamicMaterialInstance (Variables|MyProjectile|GetSphere) 0 "/Game/Materials/Projectiles/M_Projectile.M_Projectile" :!class /Script/Engine.PrimitiveComponent))
  (Variables|Default|SetProjectileMaterial _returnvalue)
  ;;[1 1 1] Get Player
  (bind _outactors (Actor|GetAllActorsOfClass "/Game/Blueprints/BP_Character.BP_Character_C"))
  (Variables|Default|SetPlayer (Utilities|Array|Get(acopy) _outactors))
  (|ChangeColor))

(event Collision|EventHit
  (params (MyComp :type Primitive%20Component%20Object%20Reference) (Other :type Actor%20Object%20Reference) (OtherComp :type Primitive%20Component%20Object%20Reference) (bSelfMoved :type Boolean) (HitLocation :type Vector :default "0, 0, 0") (HitNormal :type Vector :default "0, 0, 0") (NormalImpulse :type Vector :default "0, 0, 0") (Hit :type Hit%20Result%20Structure%20%28by%20ref%29))
  ;[1 1 1] Destroy On Hit
  (Utilities|FlowControl|Delay 0.01)
  (Actor|DestroyActor))

(fn ConstructionScript)