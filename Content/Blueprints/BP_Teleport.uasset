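; Teleporter actor that moves player character 0 to a point 150 units above a referenced Target actor.
; Its Box overlap sets CanTeleport on the overlapping BP_Character and its own IsActive flag, clearing both on exit.
; The OnTeleport event does the move without checking either flag, behind a DoOnce that stays closed until ResetTP reopens it.
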(event OnComponentBeginOverlap(Box)
  (params (OverlappedComponent :type Primitive%20Component%20Object%20Reference) (OtherActor :type Actor%20Object%20Reference) (OtherComp :type Primitive%20Component%20Object%20Reference) (OtherBodyIndex :type Integer) (bFromSweep :type Boolean) (SweepResult :type Hit%20Result%20Structure%20%28by%20ref%29))
  (bind _asbp_character (Utilities|Casting|CastToBP_Character OtherActor))
  (Variables|/Game/Blueprints/BP_Character.BP_Character_C|SetCanTeleport _asbp_character true)
  (Variables|Default|SetIsActive true))

(event OnComponentEndOverlap(Box)
  (params (OverlappedComponent :type Primitive%20Component%20Object%20Reference) (OtherActor :type Actor%20Object%20Reference) (OtherComp :type Primitive%20Component%20Object%20Reference) (OtherBodyIndex :type Integer))
  (bind _asbp_character (Utilities|Casting|CastToBP_Character OtherActor))
  (Variables|/Game/Blueprints/BP_Character.BP_Character_C|SetCanTeleport _asbp_character false)
  (Variables|Default|SetIsActive false))

(event Custom|Reset%20TP
  (bind _target (Variables|Default|GetTarget))
  (bind _returnvalue (Transformation|GetActorLocation _target))
  (bind (_x _y _z) (Math|Vector|BreakVector _returnvalue))
  (Utilities|FlowControl|DoOnce false) ; enters at Reset
)

(event Custom|OnTeleport
  (bind _target (Variables|Default|GetTarget))
  (bind _returnvalue (Transformation|GetActorLocation _target))
  (bind (_x _y _z) (Math|Vector|BreakVector _returnvalue))
  (Utilities|FlowControl|DoOnce false
    (:Completed
      (Transformation|SetActorLocation (Game|GetPlayerCharacter 0) (Math|Vector|MakeVector _x _y (+ _z 1.5e+02)) false true))))

(fn ConstructionScript)