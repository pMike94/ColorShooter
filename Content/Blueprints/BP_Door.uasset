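; BP_Door is a sliding door that opens automatically for enemies and closes behind them.
; Overlaps on the OpenDoor_Trigger component play or reverse the Door_TL timeline, ignoring any actor that is not a BP_Enemy.
; The timeline slides the Bottom panel along local Z and the Left and Right panels apart along X, mirroring one curve.
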(event OnComponentBeginOverlap(OpenDoor_Trigger)
  (params (OverlappedComponent :type Primitive%20Component%20Object%20Reference) (OtherActor :type Actor%20Object%20Reference) (OtherComp :type Primitive%20Component%20Object%20Reference) (OtherBodyIndex :type Integer) (bFromSweep :type Boolean) (SweepResult :type Hit%20Result%20Structure%20%28by%20ref%29))
  (Utilities|Casting|CastToBP_Enemy OtherActor)
  (bind (_direction _bottom _leftright) (Timeline|Door_TL Play)
    (:Update
      (Transformation|SetRelativeLocation (Variables|Default|GetBottom) (Math|Vector|MakeVector 0.0 0.0 _bottom) false false)
      (Transformation|SetRelativeLocation (Variables|Default|GetRight) (Math|Vector|MakeVector _leftright 0.0 0.0) false false)
      (Transformation|SetRelativeLocation (Variables|Default|GetLeft) (Math|Vector|MakeVector (* _leftright -1.0) 0.0 0.0) false false))))

(event OnComponentEndOverlap(OpenDoor_Trigger)
  (params (OverlappedComponent :type Primitive%20Component%20Object%20Reference) (OtherActor :type Actor%20Object%20Reference) (OtherComp :type Primitive%20Component%20Object%20Reference) (OtherBodyIndex :type Integer))
  (Utilities|Casting|CastToBP_Enemy OtherActor)
  (bind (_direction _bottom _leftright) (Timeline|Door_TL Reverse)
    (:Update
      (Transformation|SetRelativeLocation (Variables|Default|GetBottom) (Math|Vector|MakeVector 0.0 0.0 _bottom) false false)
      (Transformation|SetRelativeLocation (Variables|Default|GetRight) (Math|Vector|MakeVector _leftright 0.0 0.0) false false)
      (Transformation|SetRelativeLocation (Variables|Default|GetLeft) (Math|Vector|MakeVector (* _leftright -1.0) 0.0 0.0) false false))))

(fn ConstructionScript)